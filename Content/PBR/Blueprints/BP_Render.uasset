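; Material preview pawn that displays a mesh for scene capture and opens the UI_Main widget.
; Owner-no-see hides the mesh from the player's view, leaving it visible to the capture.
; Mouse input drives controller yaw/pitch and smoothly zooms spring arm length or ortho width, depending on projection type.
; Construction bakes Voronoi and base materials into render targets and creates a dynamic material, with functions to swap textures, normals and mesh.
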(event Custom|BakeTexture
  (Rendering|DrawMaterialtoRenderTarget "/Game/PBR/RenderTarget/RT_Voronoi_Inverted.RT_Voronoi_Inverted" "/Game/PBR/Materials/M_VoronoiInverted.M_VoronoiInverted")
  (Rendering|DrawMaterialtoRenderTarget "/Game/PBR/RenderTarget/RT_Voronoi_Highpass.RT_Voronoi_Highpass" "/Game/PBR/Materials/M_VoronoiHighpass.M_VoronoiHighpass")
  (Rendering|DrawMaterialtoRenderTarget "/Game/PBR/RenderTarget/RT_Voronoi_NormalMap.RT_Voronoi_NormalMap" "/Game/PBR/Materials/M_VoronoiNormal.M_VoronoiNormal")
  (Rendering|DrawMaterialtoRenderTarget "/Game/PBR/RenderTarget/RT_Voronoi_Final.RT_Voronoi_Final" "/Game/PBR/Materials/M_ObjectBase.M_ObjectBase"))

(event EventBeginPlay
  ;[0 0 0] Se o "owner" deste objeto for o pawn, marcar "owner no see" fará com que o objeto não apareça no mundo para o "pawn". Queremos isso para que apenas o scene capture possa visualizar por meio do material gerado (imagem que vemos na interface).
  (Actor|SetOwner (Game|Player|GetPlayerPawn 0))
  (Class|PrimitiveComponent|SetOwnerNoSee (Variables|Default|GetMesh) true)
  (Variables|/Script/Engine.PlayerController|SetbShowMouseCursor (Game|GetPlayerController 0) true)
  (bind _returnvalue (UserInterface|CreateWidget "/Game/PBR/Widgets/UI_Main.UI_Main_C"))
  (UserInterface|Viewport|AddtoViewport _returnvalue 0))

(event Collision|EventActorBeginOverlap
  (params (OtherActor :type Actor%20Object%20Reference)))

(event EventTick
  (params (DeltaSeconds :type Float%20%28single-precision%29))
  (|Zoomupdate DeltaSeconds))

(event Input|MouseEvents|MouseWheelAxis
  (params (AxisValue :type Float%20%28single-precision%29))
  ;[0 0 0] Zoom in/out
  (switch int (Math|Conversions|ToInteger(Byte) (Variables|/Script/Engine.SceneCaptureComponent2D|GetProjectionType (Variables|Default|GetSceneCaptureComponent2D)))
    (:0
      (Variables|Default|SetCurrentTargetLength (+ (Variables|Default|GetCurrentTargetLength) (* AxisValue -1.0 (Variables|Default|GetZoomSensitivity)))))
    (:1
      (Variables|Default|SetCurrentOrthoWidth (+ (Variables|/Script/Engine.SceneCaptureComponent2D|GetOrthoWidth (Variables|Default|GetSceneCaptureComponent2D)) (* AxisValue -1.0 (Variables|Default|GetZoomSensitivity)))))))

(event Input|MouseEvents|MouseX
  (params (AxisValue :type Float%20%28single-precision%29))
  (Pawn|Input|AddControllerYawInput AxisValue))

(event Input|MouseEvents|MouseY
  (params (AxisValue :type Float%20%28single-precision%29))
  (Pawn|Input|AddControllerPitchInput (* AxisValue -1.0)))

(fn ConstructionScript
  ;[1 1 1] Define o valor padrão inicial do spring arm length e ortho width.
  (Variables|Default|SetCurrentTargetLength (Variables|/Script/Engine.SpringArmComponent|GetTargetArmLength (Variables|Default|GetSpringArm)))
  (Variables|Default|SetCurrentOrthoWidth (Variables|/Script/Engine.SceneCaptureComponent2D|GetOrthoWidth (Variables|Default|GetSceneCaptureComponent2D)))
  (bind _returnvalue (Rendering|Material|CreateDynamicMaterialInstance "/Game/PBR/Materials/M_ObjectBase.M_ObjectBase" "None" "None" :!class /Script/Engine.KismetMaterialLibrary))
  (bind _output_get (Variables|Default|SetDynamicMaterialReference _returnvalue))
  (Rendering|Material|SetMaterial (Variables|Default|GetMesh) 0 _output_get)
  (Rendering|LOD|SetForcedLodModel (Variables|Default|GetMesh) 0)
  (CallFunction|BakeTexture))

(fn UpdateMaterialTexture
  (params (Texture :type Texture%20Object%20Reference))
  (Rendering|Material|SetTextureParameterValue (Variables|Default|GetDynamicMaterialReference) "Texture" Texture))

(fn UpdateMaterialNormal
  (params (Texture :type Texture%20Object%20Reference))
  (Rendering|Material|SetTextureParameterValue (Variables|Default|GetDynamicMaterialReference) "Normal" Texture))

(fn UpdateMesh
  (params (NewMesh :type Static%20Mesh%20Object%20Reference))
  (Components|StaticMesh|SetStaticMesh (Variables|Default|GetMesh) NewMesh)
  (Rendering|Material|SetMaterial (Variables|Default|GetMesh) 0 (Variables|Default|GetDynamicMaterialReference)))