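; Demo actor that builds a grid of meshes showing how metallic and roughness values affect a material.
; The construction script adds a static mesh component per MatrixSize cell in the XZ plane, each with a dynamic instance of M_BasicMaterial.
; Roughness rises in tenths along Z and Metallic rises in tenths along X.
; On BeginPlay, the actor makes itself the first player controller's view target.
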(event EventBeginPlay
  (Game|Player|SetViewTargetwithBlend (Game|GetPlayerController 0) self 0.0 "VTBlend_Linear" 0.0 false))

(fn ConstructionScript
  (bind _matrixsize (Variables|Default|GetMatrixSize))
  (for _index (range 0 (- (.x _matrixsize) 1))
    (for _index_2 (range 0 (- (.y _matrixsize) 1))
      (bind _returnvalue (AddComponent|AddStaticMeshComponent false (Math|Transform|MakeTransform (Math|Vector|MakeVector (Math|Conversions|ToFloat(Integer) (* _index_2 110)) 0.0 (Math|Conversions|ToFloat(Integer) (* _index 110))) "0, 0, 0" "1.000000,1.000000,1.000000")))
      (bind _returnvalue_2 (Rendering|Material|CreateDynamicMaterialInstance _returnvalue 0 "/Game/M_BasicMaterial.M_BasicMaterial" "None" :!class /Script/Engine.PrimitiveComponent))
      (Rendering|Material|SetScalarParameterValue _returnvalue_2 "Roughness" (/ (Math|Conversions|ToFloat(Integer) _index) 1e+01) :!class /Script/Engine.MaterialInstanceDynamic)
      (Rendering|Material|SetScalarParameterValue _returnvalue_2 "Metallic" (/ (Math|Conversions|ToFloat(Integer) _index_2) 1e+01) :!class /Script/Engine.MaterialInstanceDynamic)
      (Rendering|Material|SetMaterial _returnvalue 0 _returnvalue_2))))